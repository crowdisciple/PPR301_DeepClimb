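; BP_Checkpoint is an ordered checkpoint actor that records its transform as the player character's respawn-style CurrentCheckpoint.
; OrderNum 0 sets the default on BeginPlay, when an optional coral sapling sprite is also shown.
; Box overlaps advance the checkpoint only in checkpoint mode and for a higher OrderNum.
; A Sense collider starts a looping timer that smoothly yaws the actor toward the overlapping Character until overlap ends.
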(event OnComponentBeginOverlap(Box)
  (params (OverlappedComponent :type Primitive%20Component%20Object%20Reference) (OtherActor :type Actor%20Object%20Reference) (OtherComp :type Primitive%20Component%20Object%20Reference) (OtherBodyIndex :type Integer) (bFromSweep :type Boolean) (SweepResult :type Hit%20Result%20Structure%20%28by%20ref%29))
  (bind _asbp_first_person_character (Utilities|Casting|CastToBP_FirstPersonCharacter (Game|GetPlayerCharacter 0)))
  (if (Variables|/Game/FirstPerson/Blueprints/BP_FirstPersonCharacter.BP_FirstPersonCharacter_C|GetCheckpointModeOn? _asbp_first_person_character)
    (if (> (Variables|Default|GetOrderNum) (Variables|/Game/FirstPerson/Blueprints/BP_FirstPersonCharacter.BP_FirstPersonCharacter_C|GetCheckpointInt _asbp_first_person_character))
      (Variables|/Game/FirstPerson/Blueprints/BP_FirstPersonCharacter.BP_FirstPersonCharacter_C|SetCheckpointInt _asbp_first_person_character (Variables|Default|GetOrderNum))
      (Variables|/Game/FirstPerson/Blueprints/BP_FirstPersonCharacter.BP_FirstPersonCharacter_C|SetCurrent%20Checkpoint _asbp_first_person_character (Transformation|GetActorTransform)))))

(event OnComponentBeginOverlap(Sense)
  (params (OverlappedComponent :type Primitive%20Component%20Object%20Reference) (OtherActor :type Actor%20Object%20Reference) (OtherComp :type Primitive%20Component%20Object%20Reference) (OtherBodyIndex :type Integer) (bFromSweep :type Boolean) (SweepResult :type Hit%20Result%20Structure%20%28by%20ref%29))
  ;[1 1 1] Identify when an actor overlaps the sense collider and makes a reference of them
  (bind _ascharacter (Utilities|Casting|CastToCharacter OtherActor))
  (Variables|Default|SetChar%20REF _ascharacter)
  (bind _returnvalue (Utilities|Time|SetTimerbyEvent (delegate Custom|Rotate) 0.01 true))
  (Variables|Default|SetTimer%20Handle _returnvalue))

(event OnComponentEndOverlap(Sense)
  (params (OverlappedComponent :type Primitive%20Component%20Object%20Reference) (OtherActor :type Actor%20Object%20Reference) (OtherComp :type Primitive%20Component%20Object%20Reference) (OtherBodyIndex :type Integer))
  ;[1 1 1] Ends rotation when the actor leaves the collider
  (Utilities|Time|ClearandInvalidateTimerbyHandle (Variables|Default|GetTimer%20Handle)))

(event Custom|Rotate
  ;[1 1 1] Makes the actor face the pawn that overlapped the collision
  (Transformation|SetActorRotation (Math|Rotator|MakeRotator 0.0 0.0 (.yaw (Math|Interpolation|RInterpTo (Transformation|GetActorRotation) (Math|Rotator|FindLookatRotation (Transformation|GetActorLocation) (Transformation|GetActorLocation (Variables|Default|GetChar%20REF))) (Utilities|Time|GetWorldDeltaSeconds) 1e+01)))))

(event EventBeginPlay
  ;[0.4852 0.956 1] On BeginPlay this checks if OrderNum == 0, and if so it will be set as the first default checkpoint. (If multiple are set to 0 it goes to the most recently added)
  (if (== (Variables|Default|GetOrderNum) 0)
    (bind _asbp_first_person_character (Utilities|Casting|CastToBP_FirstPersonCharacter (Game|GetPlayerCharacter 0)))
    (Variables|/Game/FirstPerson/Blueprints/BP_FirstPersonCharacter.BP_FirstPersonCharacter_C|SetCurrent%20Checkpoint _asbp_first_person_character (Transformation|GetActorTransform)))
  (if (Variables|Default|GetVisible?)
    (Rendering|SetVisibility (Variables|Default|GetCoral_Sapling_Sprite) true false)))

(fn ConstructionScript)