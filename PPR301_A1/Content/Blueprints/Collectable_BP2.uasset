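; Collectable actor that opens a text screen when interacted with, switching to Game and UI input with a visible cursor and flagging the first-person character as reading.
; A collision sphere shows and hides the interaction prompt widget on overlap.
; A separate Sense collider stores the overlapping Character and runs a looping timer that smoothly turns the collectable's yaw toward them, clearing it on end overlap.
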(event OnComponentBeginOverlap(Spherecollision)
  (params (OverlappedComponent :type Primitive%20Component%20Object%20Reference) (OtherActor :type Actor%20Object%20Reference) (OtherComp :type Primitive%20Component%20Object%20Reference) (OtherBodyIndex :type Integer) (bFromSweep :type Boolean) (SweepResult :type Hit%20Result%20Structure%20%28by%20ref%29))
  ;[0.4852 0.956 1] Show/Hide interaction prompt visibility
  (Rendering|SetVisibility (Variables|Default|GetInteractionPromptWidget) true false))

(event OnComponentEndOverlap(Spherecollision)
  (params (OverlappedComponent :type Primitive%20Component%20Object%20Reference) (OtherActor :type Actor%20Object%20Reference) (OtherComp :type Primitive%20Component%20Object%20Reference) (OtherBodyIndex :type Integer))
  ;[0.4852 0.956 1] Show/Hide interaction prompt visibility
  (Rendering|SetVisibility (Variables|Default|GetInteractionPromptWidget) false false))

(event OnComponentBeginOverlap(Sense)
  (params (OverlappedComponent :type Primitive%20Component%20Object%20Reference) (OtherActor :type Actor%20Object%20Reference) (OtherComp :type Primitive%20Component%20Object%20Reference) (OtherBodyIndex :type Integer) (bFromSweep :type Boolean) (SweepResult :type Hit%20Result%20Structure%20%28by%20ref%29))
  ;[1 1 1] Identify when an actor overlaps the sense collider and makes a reference of them
  (bind _ascharacter (Utilities|Casting|CastToCharacter OtherActor))
  (Variables|Default|SetChar%20REF _ascharacter)
  (bind _returnvalue (Utilities|Time|SetTimerbyEvent (delegate Custom|Rotate) 0.01 true))
  (Variables|Default|SetTimer%20Handle _returnvalue))

(event OnComponentEndOverlap(Sense)
  (params (OverlappedComponent :type Primitive%20Component%20Object%20Reference) (OtherActor :type Actor%20Object%20Reference) (OtherComp :type Primitive%20Component%20Object%20Reference) (OtherBodyIndex :type Integer))
  ;[1 1 1] Ends rotation when the actor leaves the collider
  (Utilities|Time|ClearandInvalidateTimerbyHandle (Variables|Default|GetTimer%20Handle)))

(event Custom|Rotate
  ;[1 1 1] Makes the actor face the pawn that overlapped the collision
  (Transformation|SetActorRotation (Math|Rotator|MakeRotator 0.0 0.0 (.yaw (Math|Interpolation|RInterpTo (Transformation|GetActorRotation) (Math|Rotator|FindLookatRotation (Transformation|GetActorLocation) (Transformation|GetActorLocation (Variables|Default|GetChar%20REF))) (Utilities|Time|GetWorldDeltaSeconds) 1e+01)))))

(event EventInteract
  (bind _returnvalue (Game|GetPlayerController 0))
  ;[0.4852 0.956 1] Opens collectable text UI when interacted with
  (bind _returnvalue_2 (UserInterface|CreateWidget "/Game/UI/Collectable_ScreenWB_02.Collectable_ScreenWB_02_C" _returnvalue))
  (bind _output_get (Variables|Default|SetCollectable%20Text%20WB%202 _returnvalue_2))
  (UserInterface|Viewport|AddtoViewport _output_get 0)
  (Input|SetInputModeGameandUI _returnvalue (Variables|Default|GetCollectable%20Text%20WB%202) "DoNotLock" true false)
  (Variables|/Script/Engine.PlayerController|SetbShowMouseCursor (Game|GetPlayerController 0) true)
  (bind _asbp_first_person_character (Utilities|Casting|CastToBP_FirstPersonCharacter (Game|GetPlayerCharacter 0)))
  (Variables|/Game/FirstPerson/Blueprints/BP_FirstPersonCharacter.BP_FirstPersonCharacter_C|SetisReading? _asbp_first_person_character true))

(fn ConstructionScript)