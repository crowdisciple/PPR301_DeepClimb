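; BP_Boundary is a boundary volume that pushes the first-person character along a set direction while it overlaps the trigger.
; Begin overlap sets an out-of-bounds flag and starts a short-delay loop that adds the Arrow component's forward vector, scaled, to the character's movement velocity.
; End overlap by the character clears the flag, which ends the loop after its next push.
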(event OnComponentBeginOverlap(BoundaryTrigger)
  (params (OverlappedComponent :type Primitive%20Component%20Object%20Reference) (OtherActor :type Actor%20Object%20Reference) (OtherComp :type Primitive%20Component%20Object%20Reference) (OtherBodyIndex :type Integer) (bFromSweep :type Boolean) (SweepResult :type Hit%20Result%20Structure%20%28by%20ref%29))
  (bind _asbp_first_person_character (Utilities|Casting|CastToBP_FirstPersonCharacter OtherActor))
  (Variables|Default|SetIsOutofBounds? true)
  (Utilities|FlowControl|Delay 0.01 :!label _label)
  (Variables|/Script/Engine.MovementComponent|SetVelocity (Variables|/Script/Engine.Character|GetCharacterMovement _asbp_first_person_character) (+ (* (Math|Vector|GetForwardVector (Variables|Default|GetArrow)) "100.000000,100.000000,100.000000") (Variables|/Script/Engine.MovementComponent|GetVelocity (Variables|/Script/Engine.Character|GetCharacterMovement _asbp_first_person_character))))
  (if (Variables|Default|GetIsOutofBounds?)
    (goto _label)))

(event OnComponentEndOverlap(BoundaryTrigger)
  (params (OverlappedComponent :type Primitive%20Component%20Object%20Reference) (OtherActor :type Actor%20Object%20Reference) (OtherComp :type Primitive%20Component%20Object%20Reference) (OtherBodyIndex :type Integer))
  (Utilities|Casting|CastToBP_FirstPersonCharacter OtherActor)
  (Variables|Default|SetIsOutofBounds? false))

(event EventBeginPlay)

(event Collision|EventActorBeginOverlap
  (params (OtherActor :type Actor%20Object%20Reference)))

(event EventTick
  (params (DeltaSeconds :type Float%20%28single-precision%29)))

(fn ConstructionScript)