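; BP_ArrowSpline animates an arrowhead sprite and an FX dot travelling along its spline at a set speed.
; Tick accumulates distance and applies the spline's local location and rotation to both components, using the sprite's scale.
; With looping on, passing the spline's end resets the distance and hides only the arrowhead.
; A flag then routes Tick into a delay that pauses movement before re-showing it.
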(event EventTick
  (params (DeltaSeconds :type Float%20%28single-precision%29))
  (if (Variables|Default|GetDelay)
    (Utilities|FlowControl|Delay (Variables|Default|GetLoop%20Delay))
    (Variables|Default|SetDelay false)
    (Rendering|SetVisibility (Variables|Default|GetArrowhead_Sprite) true false)
    (else
      (Variables|Default|SetDistance%20Along%20Spline (+ (* DeltaSeconds (Variables|Default|GetSpline%20Speed)) (Variables|Default|GetDistance%20Along%20Spline)))
      (Transformation|SetRelativeTransform (Variables|Default|GetFX_ArrowDot) (Math|Transform|MakeTransform (.location (Spline|GetTransformatDistanceAlongSpline (Variables|Default|GetSpline) (Variables|Default|GetDistance%20Along%20Spline) "Local" false)) (.rotation (Spline|GetTransformatDistanceAlongSpline (Variables|Default|GetSpline) (Variables|Default|GetDistance%20Along%20Spline) "Local" false)) (Variables|/Script/Engine.SceneComponent|GetRelativeScale3D (Variables|Default|GetArrowhead_Sprite))) false false)
      (if (Variables|Default|GetLoop?)
        (if (> (Variables|Default|GetDistance%20Along%20Spline) (Spline|GetSplineLength (Variables|Default|GetSpline)))
          (Variables|Default|SetDistance%20Along%20Spline 0.0)
          (Variables|Default|SetDelay true)
          (Rendering|SetVisibility (Variables|Default|GetArrowhead_Sprite) false false))))))

(fn ConstructionScript)