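; BP_Ending is a trigger box that shows an ending screen on overlap, with the variant chosen by EndingVersionInt.
; The normal ending only adds Ending_TextWB to the viewport.
; The Jump, JOLT and VAULT tutorial endings add TutorialEnding_TextWB, show the cursor with game-and-UI input, disable first-person character input and start that widget's matching ending sequence.
; The overlap does not filter which actor entered.
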(event OnComponentBeginOverlap(Box)
  (params (OverlappedComponent :type Primitive%20Component%20Object%20Reference) (OtherActor :type Actor%20Object%20Reference) (OtherComp :type Primitive%20Component%20Object%20Reference) (OtherBodyIndex :type Integer) (bFromSweep :type Boolean) (SweepResult :type Hit%20Result%20Structure%20%28by%20ref%29))
  ;[0.4852 0.956 1] 0 = Normal Ending, 1 = Jump Ending, 2 = JOLT Ending, 3 = VAULT Ending
  (if (== (Variables|Default|GetEndingVersionInt) 0)
    (bind _returnvalue (UserInterface|CreateWidget "/Game/UI/Ending_TextWB.Ending_TextWB_C"))
    (UserInterface|Viewport|AddtoViewport _returnvalue 0)
    (elif (== (Variables|Default|GetEndingVersionInt) 1)
      (bind _returnvalue_2 (UserInterface|CreateWidget "/Game/UI/TutorialEnding_TextWB.TutorialEnding_TextWB_C"))
      (UserInterface|Viewport|AddtoViewport _returnvalue_2 0)
      (Input|SetInputModeGameandUI (Game|GetPlayerController 0) (Variables|Default|GetTutorialEndingWB) "DoNotLock" true false)
      (Variables|/Script/Engine.PlayerController|SetbShowMouseCursor (Game|GetPlayerController 0) true)
      (bind _asbp_first_person_character (Utilities|Casting|CastToBP_FirstPersonCharacter (Game|GetPlayerCharacter 0)))
      (Input|DisableInput _asbp_first_person_character 0)
      (Default|StartJumpEnding _returnvalue_2)
      (elif (== (Variables|Default|GetEndingVersionInt) 2)
        (bind _returnvalue_3 (UserInterface|CreateWidget "/Game/UI/TutorialEnding_TextWB.TutorialEnding_TextWB_C"))
        (UserInterface|Viewport|AddtoViewport _returnvalue_3 0)
        (Input|SetInputModeGameandUI (Game|GetPlayerController 0) (Variables|Default|GetTutorialEndingWB) "DoNotLock" true false)
        (Variables|/Script/Engine.PlayerController|SetbShowMouseCursor (Game|GetPlayerController 0) true)
        (bind _asbp_first_person_character_2 (Utilities|Casting|CastToBP_FirstPersonCharacter (Game|GetPlayerCharacter 0)))
        (Input|DisableInput _asbp_first_person_character_2 0)
        (Default|StartJOLTEnding _returnvalue_3)
        (elif (== (Variables|Default|GetEndingVersionInt) 3)
          (bind _returnvalue_4 (UserInterface|CreateWidget "/Game/UI/TutorialEnding_TextWB.TutorialEnding_TextWB_C"))
          (UserInterface|Viewport|AddtoViewport _returnvalue_4 0)
          (Input|SetInputModeGameandUI (Game|GetPlayerController 0) (Variables|Default|GetTutorialEndingWB) "DoNotLock" true false)
          (Variables|/Script/Engine.PlayerController|SetbShowMouseCursor (Game|GetPlayerController 0) true)
          (bind _asbp_first_person_character_3 (Utilities|Casting|CastToBP_FirstPersonCharacter (Game|GetPlayerCharacter 0)))
          (Input|DisableInput _asbp_first_person_character_3 0)
          (Default|StartEnding _returnvalue_4))))))

(fn ConstructionScript)