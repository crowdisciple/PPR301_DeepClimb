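; Readable collectable pickup that shows a sprite and opens a text screen, both chosen by CollectableTextInt.
; A sphere overlap toggles the prompt and range flag that gate IA_Interact.
; Interacting opens the widget, disables character movement, flags reading and hides the aura, recording first reads in the character's collectable array and count.
; A Sense overlap starts a looping timer that yaws the actor toward the character; end overlap never clears it.
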(event OnComponentBeginOverlap(Spherecollision)
  (params (OverlappedComponent :type Primitive%20Component%20Object%20Reference) (OtherActor :type Actor%20Object%20Reference) (OtherComp :type Primitive%20Component%20Object%20Reference) (OtherBodyIndex :type Integer) (bFromSweep :type Boolean) (SweepResult :type Hit%20Result%20Structure%20%28by%20ref%29))
  ;[0.4852 0.956 1] Show/Hide interaction prompt visibility
  (Rendering|SetVisibility (Variables|Default|GetInteractionPromptWidget) true false)
  ;[0.4852 0.956 1] Sets if 'Can Interact?' is true or false at the same time as the prompt.
  (bind _asbp_first_person_character (Utilities|Casting|CastToBP_FirstPersonCharacter (Game|GetPlayerCharacter 0)))
  ;;[1 1 1 1 14] There are two variables here that are essentially the same because one is from the Character BP, and is used by the other interaction systems I tried
  (Variables|/Game/FirstPerson/Blueprints/BP_FirstPersonCharacter.BP_FirstPersonCharacter_C|SetCanInteract? _asbp_first_person_character true)
  (Variables|Default|SetInInteractionRange? true))

(event OnComponentEndOverlap(Spherecollision)
  (params (OverlappedComponent :type Primitive%20Component%20Object%20Reference) (OtherActor :type Actor%20Object%20Reference) (OtherComp :type Primitive%20Component%20Object%20Reference) (OtherBodyIndex :type Integer))
  ;[0.4852 0.956 1] Show/Hide interaction prompt visibility
  (Rendering|SetVisibility (Variables|Default|GetInteractionPromptWidget) false false)
  ;[0.4852 0.956 1] Sets if 'Can Interact?' is true or false at the same time as the prompt.
  (bind _asbp_first_person_character (Utilities|Casting|CastToBP_FirstPersonCharacter (Game|GetPlayerCharacter 0)))
  ;;[1 1 1 1 14] There are two variables here that are essentially the same because one is from the Character BP, and is used by the other interaction systems I tried
  (Variables|/Game/FirstPerson/Blueprints/BP_FirstPersonCharacter.BP_FirstPersonCharacter_C|SetCanInteract? _asbp_first_person_character false)
  (Variables|Default|SetInInteractionRange? false))

(event OnComponentBeginOverlap(Sense)
  (params (OverlappedComponent :type Primitive%20Component%20Object%20Reference) (OtherActor :type Actor%20Object%20Reference) (OtherComp :type Primitive%20Component%20Object%20Reference) (OtherBodyIndex :type Integer) (bFromSweep :type Boolean) (SweepResult :type Hit%20Result%20Structure%20%28by%20ref%29))
  ;[1 1 1] Identify when an actor overlaps the sense collider and makes a reference of them
  (bind _ascharacter (Utilities|Casting|CastToCharacter OtherActor))
  (Variables|Default|SetChar%20REF _ascharacter)
  (bind _returnvalue (Utilities|Time|SetTimerbyEvent (delegate Custom|Rotate) 0.01 true))
  (Variables|Default|SetTimer%20Handle _returnvalue))

(event OnComponentEndOverlap(Sense)
  (params (OverlappedComponent :type Primitive%20Component%20Object%20Reference) (OtherActor :type Actor%20Object%20Reference) (OtherComp :type Primitive%20Component%20Object%20Reference) (OtherBodyIndex :type Integer))
  ;[1 1 1] Ends rotation when the actor leaves the collider
)

(event Custom|Rotate
  ;[1 1 1] Makes the actor face the pawn that overlapped the collision
  (Transformation|SetActorRotation (Math|Rotator|MakeRotator 0.0 0.0 (.yaw (Math|Interpolation|RInterpTo (Transformation|GetActorRotation) (Math|Rotator|FindLookatRotation (Transformation|GetActorLocation) (Transformation|GetActorLocation (Variables|Default|GetChar%20REF))) (Utilities|Time|GetWorldDeltaSeconds) 1e+01)))))

(event Input|EnhancedActionEvents|EnhancedInputActionIA_Interact
  (params (ActionValue :type Boolean) (ElapsedSeconds :type Float%20%28double-precision%29) (TriggeredSeconds :type Float%20%28double-precision%29) (InputAction :type Input%20Action%20Object%20Reference :default "/Game/FirstPerson/Input/Actions/IA_Interact.IA_Interact"))
  (bind _returnvalue (Game|GetPlayerController 0))
  (bind _returnvalue_2 (Game|GetPlayerCharacter 0))
  (bind _returnvalue_3 (Game|GetPlayerController 0))
  (bind _collectabletext_int (Variables|Default|GetCollectableText_int))
  ;[0.4852 0.956 1] Opens the WB that matches the specified text.
  (if (Variables|Default|GetInInteractionRange?)
    (bind _asbp_first_person_character (Utilities|Casting|CastToBP_FirstPersonCharacter (Game|GetPlayerCharacter 0)))
    (if (not (Variables|/Game/FirstPerson/Blueprints/BP_FirstPersonCharacter.BP_FirstPersonCharacter_C|GetisReading? _asbp_first_person_character))
      (Widget|SetVisibility (Variables|/Game/FirstPerson/Blueprints/BP_FirstPersonCharacter.BP_FirstPersonCharacter_C|GetJumpChargeWB%20REF _asbp_first_person_character) "Collapsed")
      (if (== _collectabletext_int 1)
        ;[0.4852 0.956 1] Opens collectable text UI when interacted with
        (bind _returnvalue_4 (UserInterface|CreateWidget "/Game/UI/Collectable_ScreenWB_01_CannedAir.Collectable_ScreenWB_01_CannedAir_C" _returnvalue))
        (bind _output_get (Variables|Default|SetCollectableTextWB_01 _returnvalue_4))
        (UserInterface|Viewport|AddtoViewport _output_get 0)
        (Input|SetInputModeGameandUI _returnvalue_3 (Variables|Default|GetCollectableTextWB_01) "DoNotLock" true false)
        (if (Variables|Default|GetCollectable%201%20Counted?)
          _
          (else
            (bind _output_get_2 (Variables|Default|SetCollectable%201%20Counted? true))
            (bind _asbp_first_person_character_2 (Utilities|Casting|CastToBP_FirstPersonCharacter _returnvalue_2))
            (Utilities|Array|Insert (Variables|/Game/FirstPerson/Blueprints/BP_FirstPersonCharacter.BP_FirstPersonCharacter_C|GetCollectable%20Array _asbp_first_person_character_2) _output_get_2 1)
            (bind _asbp_first_person_character_3 (Utilities|Casting|CastToBP_FirstPersonCharacter (Game|GetPlayerCharacter 0) :!label _label))
            (Variables|/Game/FirstPerson/Blueprints/BP_FirstPersonCharacter.BP_FirstPersonCharacter_C|SetCollectable%20Count _asbp_first_person_character_3 (+ (Variables|/Game/FirstPerson/Blueprints/BP_FirstPersonCharacter.BP_FirstPersonCharacter_C|GetCollectable%20Count _asbp_first_person_character_3) 1))))
        (Variables|/Script/Engine.PlayerController|SetbShowMouseCursor (Game|GetPlayerController 0) true :!label _label_2)
        (bind _asbp_first_person_character_4 (Utilities|Casting|CastToBP_FirstPersonCharacter (Game|GetPlayerCharacter 0)))
        (Components|Activation|SetActive (Variables|/Script/Engine.Character|GetCharacterMovement _asbp_first_person_character_4) false false)
        (Variables|/Game/FirstPerson/Blueprints/BP_FirstPersonCharacter.BP_FirstPersonCharacter_C|SetisReading? _asbp_first_person_character_4 true)
        (Rendering|SetVisibility (Variables|Default|GetFX_CollectableAura) false false)
        (elif (== _collectabletext_int 2)
          (bind _returnvalue_5 (UserInterface|CreateWidget "/Game/UI/Collectable_ScreenWB_02_CostofAPrayer.Collectable_ScreenWB_02_CostofAPrayer_C" _returnvalue))
          (bind _output_get_3 (Variables|Default|SetCollectableTextWB_02 _returnvalue_5))
          (UserInterface|Viewport|AddtoViewport _output_get_3 0)
          (Input|SetInputModeGameandUI _returnvalue_3 (Variables|Default|GetCollectableTextWB_02) "DoNotLock" true false)
          (if (Variables|Default|GetCollectable%202%20Counted?)
            (goto _label_2)
            (else
              (bind _output_get_4 (Variables|Default|SetCollectable%202%20Counted? true))
              (bind _asbp_first_person_character_5 (Utilities|Casting|CastToBP_FirstPersonCharacter _returnvalue_2))
              (Utilities|Array|Insert (Variables|/Game/FirstPerson/Blueprints/BP_FirstPersonCharacter.BP_FirstPersonCharacter_C|GetCollectable%20Array _asbp_first_person_character_5) _output_get_4 2)
              (goto _label)))
          (elif (== _collectabletext_int 3)
            (bind _returnvalue_6 (UserInterface|CreateWidget "/Game/UI/Collectable_ScreenWB_03_Gunshot.Collectable_ScreenWB_03_Gunshot_C" _returnvalue))
            (bind _output_get_5 (Variables|Default|SetCollectableTextWB_03 _returnvalue_6))
            (UserInterface|Viewport|AddtoViewport _output_get_5 0)
            (Input|SetInputModeGameandUI _returnvalue_3 (Variables|Default|GetCollectableTextWB_03) "DoNotLock" true false)
            (if (Variables|Default|GetCollectable%203%20Counted?)
              (goto _label_2)
              (else
                (bind _output_get_6 (Variables|Default|SetCollectable%203%20Counted? true))
                (bind _asbp_first_person_character_6 (Utilities|Casting|CastToBP_FirstPersonCharacter _returnvalue_2))
                (Utilities|Array|Insert (Variables|/Game/FirstPerson/Blueprints/BP_FirstPersonCharacter.BP_FirstPersonCharacter_C|GetCollectable%20Array _asbp_first_person_character_6) _output_get_6 3)
                (goto _label)))
            (elif (== _collectabletext_int 4)
              (bind _returnvalue_7 (UserInterface|CreateWidget "/Game/UI/Collectable_ScreenWB_04_MineralMemory.Collectable_ScreenWB_04_MineralMemory_C" _returnvalue))
              (bind _output_get_7 (Variables|Default|SetCollectableTextWB_04 _returnvalue_7))
              (UserInterface|Viewport|AddtoViewport _output_get_7 0)
              (Input|SetInputModeGameandUI _returnvalue_3 (Variables|Default|GetCollectableTextWB_04) "DoNotLock" true false)
              (if (Variables|Default|GetCollectable%204%20Counted?)
                (goto _label_2)
                (else
                  (bind _output_get_8 (Variables|Default|SetCollectable%204%20Counted? true))
                  (bind _asbp_first_person_character_7 (Utilities|Casting|CastToBP_FirstPersonCharacter _returnvalue_2))
                  (Utilities|Array|Insert (Variables|/Game/FirstPerson/Blueprints/BP_FirstPersonCharacter.BP_FirstPersonCharacter_C|GetCollectable%20Array _asbp_first_person_character_7) _output_get_8 4)
                  (goto _label)))
              (elif (== _collectabletext_int 5)
                (bind _returnvalue_8 (UserInterface|CreateWidget "/Game/UI/Collectable_ScreenWB_05_Skinless.Collectable_ScreenWB_05_Skinless_C" _returnvalue))
                (bind _output_get_9 (Variables|Default|SetCollectableTextWB_05 _returnvalue_8))
                (UserInterface|Viewport|AddtoViewport _output_get_9 0)
                (Input|SetInputModeGameandUI _returnvalue_3 (Variables|Default|GetCollectableTextWB_05) "DoNotLock" true false)
                (if (Variables|Default|GetCollectable%205%20Counted?)
                  (goto _label_2)
                  (else
                    (bind _output_get_10 (Variables|Default|SetCollectable%205%20Counted? true))
                    (bind _asbp_first_person_character_8 (Utilities|Casting|CastToBP_FirstPersonCharacter _returnvalue_2))
                    (Utilities|Array|Insert (Variables|/Game/FirstPerson/Blueprints/BP_FirstPersonCharacter.BP_FirstPersonCharacter_C|GetCollectable%20Array _asbp_first_person_character_8) _output_get_10 5)
                    (goto _label)))
                (elif (== _collectabletext_int 6)
                  (bind _returnvalue_9 (UserInterface|CreateWidget "/Game/UI/Collectable_ScreenWB_06_Stargazer.Collectable_ScreenWB_06_Stargazer_C" _returnvalue))
                  (bind _output_get_11 (Variables|Default|SetCollectableTextWB_06 _returnvalue_9))
                  (UserInterface|Viewport|AddtoViewport _output_get_11 0)
                  (Input|SetInputModeGameandUI _returnvalue_3 (Variables|Default|GetCollectableTextWB_06) "DoNotLock" true false)
                  (if (Variables|Default|GetCollectable%206%20Counted?)
                    (goto _label_2)
                    (else
                      (bind _output_get_12 (Variables|Default|SetCollectable%206%20Counted? true))
                      (bind _asbp_first_person_character_9 (Utilities|Casting|CastToBP_FirstPersonCharacter _returnvalue_2))
                      (Utilities|Array|Insert (Variables|/Game/FirstPerson/Blueprints/BP_FirstPersonCharacter.BP_FirstPersonCharacter_C|GetCollectable%20Array _asbp_first_person_character_9) _output_get_12 6)
                      (goto _label)))
                  (elif (== _collectabletext_int 7)
                    (bind _returnvalue_10 (UserInterface|CreateWidget "/Game/UI/Collectable_ScreenWB_07_Pressure.Collectable_ScreenWB_07_Pressure_C" _returnvalue))
                    (bind _output_get_13 (Variables|Default|SetCollectableTextWB_07 _returnvalue_10))
                    (UserInterface|Viewport|AddtoViewport _output_get_13 0)
                    (Input|SetInputModeGameandUI _returnvalue_3 (Variables|Default|GetCollectableTextWB_07) "DoNotLock" true false)
                    (if (Variables|Default|GetCollectable%207%20Counted?)
                      (goto _label_2)
                      (else
                        (bind _output_get_14 (Variables|Default|SetCollectable%207%20Counted? true))
                        (bind _asbp_first_person_character_10 (Utilities|Casting|CastToBP_FirstPersonCharacter _returnvalue_2))
                        (Utilities|Array|Insert (Variables|/Game/FirstPerson/Blueprints/BP_FirstPersonCharacter.BP_FirstPersonCharacter_C|GetCollectable%20Array _asbp_first_person_character_10) _output_get_14 7)
                        (goto _label)))
                    (elif (== _collectabletext_int 8)
                      (bind _returnvalue_11 (UserInterface|CreateWidget "/Game/UI/Collectable_ScreenWB_08_Heartbreak.Collectable_ScreenWB_08_Heartbreak_C" _returnvalue))
                      (bind _output_get_15 (Variables|Default|SetCollectableTextWB_08 _returnvalue_11))
                      (UserInterface|Viewport|AddtoViewport _output_get_15 0)
                      (Input|SetInputModeGameandUI _returnvalue_3 (Variables|Default|GetCollectableTextWB_08) "DoNotLock" true false)
                      (if (Variables|Default|GetCollectable%208%20Counted?)
                        (goto _label_2)
                        (else
                          (bind _output_get_16 (Variables|Default|SetCollectable%208%20Counted? true))
                          (bind _asbp_first_person_character_11 (Utilities|Casting|CastToBP_FirstPersonCharacter _returnvalue_2))
                          (Utilities|Array|Insert (Variables|/Game/FirstPerson/Blueprints/BP_FirstPersonCharacter.BP_FirstPersonCharacter_C|GetCollectable%20Array _asbp_first_person_character_11) _output_get_16 8)
                          (goto _label)))
                      (elif (== _collectabletext_int 9)
                        (bind _returnvalue_12 (UserInterface|CreateWidget "/Game/UI/Collectable_ScreenWB_09_Itching.Collectable_ScreenWB_09_Itching_C"))
                        (bind _output_get_17 (Variables|Default|SetCollectableTextWB_09 _returnvalue_12))
                        (UserInterface|Viewport|AddtoViewport _output_get_17 0)
                        (Input|SetInputModeGameandUI _returnvalue_3 (Variables|Default|GetCollectableTextWB_09) "DoNotLock" true false)
                        (if (Variables|Default|GetCollectable%209%20Counted?)
                          (goto _label_2)
                          (else
                            (bind _output_get_18 (Variables|Default|SetCollectable%209%20Counted? true))
                            (bind _asbp_first_person_character_12 (Utilities|Casting|CastToBP_FirstPersonCharacter _returnvalue_2))
                            (Utilities|Array|Insert (Variables|/Game/FirstPerson/Blueprints/BP_FirstPersonCharacter.BP_FirstPersonCharacter_C|GetCollectable%20Array _asbp_first_person_character_12) _output_get_18 9)
                            (goto _label)))))))))))))))

(event EventBeginPlay
  (bind _collectabletext_int (Variables|Default|GetCollectableText_int))
  ;[0.4852 0.956 1] Enables input actions for this actor BP
  (Input|EnableInput (Game|GetPlayerController 0))
  ;[0.4852 0.956 1] Changes the sprite depending on what text is being used
  (if (== _collectabletext_int 1)
    (Rendering|SetVisibility (Variables|Default|GetPaperSprite_head) true false))
  (Rendering|SetVisibility (Variables|Default|GetPaperSprite_body) false false)
  (if (== _collectabletext_int 2)
    (Rendering|SetVisibility (Variables|Default|GetPaperSprite_head) true false)
    (elif (== _collectabletext_int 3)
      (Rendering|SetVisibility (Variables|Default|GetPaperSprite_arm) true false)
      (elif (== _collectabletext_int 4)
        (Rendering|SetVisibility (Variables|Default|GetPaperSprite_tank) true false)
        (elif (== _collectabletext_int 5)
          (Rendering|SetVisibility (Variables|Default|GetPaperSprite_body) true false)
          (elif (== _collectabletext_int 6)
            (Rendering|SetVisibility (Variables|Default|GetPaperSprite_torso) true false)
            (elif (== _collectabletext_int 7)
              (Rendering|SetVisibility (Variables|Default|GetPaperSprite_tank) true false)
              (elif (== _collectabletext_int 8)
                (Rendering|SetVisibility (Variables|Default|GetPaperSprite_torso) true false)
                (elif (== _collectabletext_int 9)
                  (Rendering|SetVisibility (Variables|Default|GetPaperSprite_arm) true false))))))))))

(fn ConstructionScript)