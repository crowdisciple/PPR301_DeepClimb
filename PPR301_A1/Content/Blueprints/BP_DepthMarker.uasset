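; BP_DepthMarker is an actor that tracks the player character's depth and shows it as debug text.
; BeginPlay seeds Depth from the player's world Z, converted from centimeters to meters with a fixed offset, then prints it in a repeating short Delay loop.
; Tick recomputes the rounded value relative to the marker's own Z and updates Depth when it changes.
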(event EventBeginPlay
  (Variables|Default|SetDepth (Class|KismetMathLibrary|ToInt64(Float) (- (/ (.z (Transformation|GetActorLocation (Game|GetPlayerCharacter 0))) 1e+02) 1147.0)))
  (Utilities|FlowControl|Delay 0.1 :!label _label)
  (Development|PrintString (Utilities|String|ToString(Integer) (Variables|Default|GetDepth)))
  (goto _label))

(event EventTick
  (params (DeltaSeconds :type Float%20%28single-precision%29))
  (bind _returnvalue (Game|GetPlayerCharacter 0))
  (bind _returnvalue_2 (Transformation|GetActorLocation))
  (bind _returnvalue_3 (Transformation|GetActorLocation _returnvalue))
  (bind _returnvalue_4 (- (.z _returnvalue_3) (.z _returnvalue_2)))
  (bind _returnvalue_5 (/ _returnvalue_4 1e+02))
  (bind _returnvalue_6 (- _returnvalue_5 1147.0))
  (bind _returnvalue_7 (Class|KismetMathLibrary|Round64 _returnvalue_6))
  (if (!= _returnvalue_7 (Variables|Default|GetDepth))
    (Variables|Default|SetDepth _returnvalue_7)))

(fn ConstructionScript)