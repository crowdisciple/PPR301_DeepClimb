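; Purple is a Blueprint with a point light that brightens and dims in response to overlaps on its CloseDetection component.
; Overlap begin plays the LightIntensity timeline at normal rate, driving the light's intensity.
; Overlap end stops the timeline, then reverses it at a slower rate after a random delay.
; Both events cast player character 0 rather than the overlapping actor, so other actors can also trigger them.
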(event OnComponentBeginOverlap(CloseDetection)
  (params (OverlappedComponent :type Primitive%20Component%20Object%20Reference) (OtherActor :type Actor%20Object%20Reference) (OtherComp :type Primitive%20Component%20Object%20Reference) (OtherBodyIndex :type Integer) (bFromSweep :type Boolean) (SweepResult :type Hit%20Result%20Structure%20%28by%20ref%29))
  (Utilities|Casting|CastToBP_FirstPersonCharacter (Game|GetPlayerCharacter 0))
  (Components|Timeline|SetPlayRate (Variables|Default|GetLightIntensity) 1.0)
  (bind _intensityvalue (Timeline|LightIntensity Play)
    (:Update
      (Rendering|Components|Light|SetIntensity (Variables|Default|GetPointLight) _intensityvalue))))

(event OnComponentEndOverlap(CloseDetection)
  (params (OverlappedComponent :type Primitive%20Component%20Object%20Reference) (OtherActor :type Actor%20Object%20Reference) (OtherComp :type Primitive%20Component%20Object%20Reference) (OtherBodyIndex :type Integer))
  (Utilities|Casting|CastToBP_FirstPersonCharacter (Game|GetPlayerCharacter 0))
  (Components|Timeline|SetPlayRate (Variables|Default|GetLightIntensity) 0.3)
  (Utilities|FlowControl|Sequence
    (:then_0
      (bind _intensityvalue (Timeline|LightIntensity Stop)
        (:Update
          (Rendering|Components|Light|SetIntensity (Variables|Default|GetPointLight) _intensityvalue))))
    (:then_1
      (Utilities|FlowControl|Delay (Math|Random|RandomFloatinRange 0.4 3.0))
      (Timeline|LightIntensity Reverse))))

(event EventBeginPlay)

(event Collision|EventActorBeginOverlap
  (params (OtherActor :type Actor%20Object%20Reference)))

(event EventTick
  (params (DeltaSeconds :type Float%20%28single-precision%29)))

(fn ConstructionScript)